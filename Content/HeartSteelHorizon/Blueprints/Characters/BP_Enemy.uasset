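; BP_Enemy is a side-scrolling flipbook fighter that, despite its name, binds player input and player flipbooks and damages BP_Player actors.
; Enhanced Input drives movement along X, jumping and a three-step attack combo.
; Tick picks locomotion flipbooks when not attacking, and on attack frame 3 fires a once-gated hitbox overlap check for damage and effects.
; AnyDamage lowers health and plays hurt or death, while finished non-death animations reset combo and idle.
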(event `self.ReceiveBeginPlay`
  (`EnhancedInputSubsystemInterface.AddMappingContext` (pcsubsystem `EnhancedInputLocalPlayerSubsystem` (`GameplayStatics.GetPlayerController` 0)) "/Game/HeartSteelHorizon/Input/IMC_Player.IMC_Player" 0 (struct)))

(event `EnhancedInput|/Game/HeartSteelHorizon/Input/IA_Move`
  (params (ActionValue :type "Float (double-precision)") (ElapsedSeconds :type "Float (double-precision)") (TriggeredSeconds :type "Float (double-precision)") (InputAction :type "InputAction Object Reference" :default "/Game/HeartSteelHorizon/Input/IA_Move.IA_Move"))
  (:`Triggered`
    (`self.AddMovementInput` (1.0 0.0 0.0) ActionValue)
    (`Controller.SetControlRotation` (`self.GetController`) (select `bool` (> ActionValue 0.0) :`false` (`KismetMathLibrary.MakeRotator` 0.0 0.0 180.0) :`true` (`KismetMathLibrary.MakeRotator` 0.0)))))

(event `EnhancedInput|/Game/HeartSteelHorizon/Input/IA_Jump`
  (params (ActionValue :type Boolean) (ElapsedSeconds :type "Float (double-precision)") (TriggeredSeconds :type "Float (double-precision)") (InputAction :type "InputAction Object Reference" :default "/Game/HeartSteelHorizon/Input/IA_Jump.IA_Jump"))
  (:`Started`
    (`self.Jump`))
  (:`Completed`
    (`self.StopJumping`)))

(event `EnhancedInput|/Game/HeartSteelHorizon/Input/IA_Attack`
  (params (ActionValue :type "Vector2D Structure") (ElapsedSeconds :type "Float (double-precision)") (TriggeredSeconds :type "Float (double-precision)") (InputAction :type "InputAction Object Reference" :default "/Game/HeartSteelHorizon/Input/IA_Attack.IA_Attack"))
  (bind _sprite (`self.Sprite`))
  (bind _sprite_2 (`self.Sprite`))
  (:`Started`
    (switch `int` (`self.ComboCount`)
      (:`Default`
        (`PaperFlipbookComponent.SetFlipbook` _sprite "/Game/HeartSteelHorizon/Sprites/Player/FlipBooks/FB_PlayerAttack1.FB_PlayerAttack1" :!label _label)
        (`PaperFlipbookComponent.SetLooping` _sprite_2 false)
        (set `self.IsAttacking` true)
        (`GameplayStatics.PlaySound2D` "/Engine/EditorSounds/GamePreview/PossessPlayer.PossessPlayer" 1.0 1.0 0.0 null null)
        (set `self.ComboCount` 1))
      (:`0`
        (goto _label))
      (:`1`
        (`PaperFlipbookComponent.SetFlipbook` _sprite "/Game/HeartSteelHorizon/Sprites/Player/FlipBooks/FB_PlayerAttack2.FB_PlayerAttack2")
        (`PaperFlipbookComponent.SetLooping` (`self.Sprite`) false)
        (`PaperFlipbookComponent.SetLooping` _sprite_2 false)
        (set `self.IsAttacking` true)
        (`GameplayStatics.PlaySound2D` "/Engine/EditorSounds/GamePreview/EndPlayInEditor.EndPlayInEditor" 1.0 1.0 0.0 null null)
        (set `self.ComboCount` 2))
      (:`2`
        (`PaperFlipbookComponent.SetFlipbook` _sprite "/Game/HeartSteelHorizon/Sprites/Player/FlipBooks/FB_PlayerAttack3.FB_PlayerAttack3")
        (`PaperFlipbookComponent.SetLooping` _sprite_2 false)
        (set `self.IsAttacking` true)
        (`GameplayStatics.PlaySound2D` "/Engine/EditorSounds/GamePreview/EjectFromPlayer.EjectFromPlayer" 1.0 1.0 0.0 null null)
        (set `self.ComboCount` 0)))))

(event `self.Sprite.OnFinishedPlaying`
  (if (not (`self.IsDead`))
    (`PaperFlipbookComponent.SetFlipbook` (`self.Sprite`) "/Game/HeartSteelHorizon/Sprites/Player/FlipBooks/FB_PlayerIdle.FB_PlayerIdle")
    (`self.RestartAnimation`)
    (set `self.IsAttacking` false)
    (`self.Reset Combo`)
    (`SceneComponent.SetHiddenInGame` (`self.Hitbox`) true false)))

(event `self.ReceiveTick`
  (params (DeltaSeconds :type "Float (single-precision)"))
  (if (`self.IsAttacking`)
    (`/Engine/EditorBlueprintResources/StandardMacros.DoOnce` false
      (:`Completed`
        (if (== (`PaperFlipbookComponent.GetPlaybackPositionInFrames` (`self.Sprite`)) 3)
          (`/Engine/EditorBlueprintResources/StandardMacros.DoOnce` false :!label _label_2
            (:`Completed`
              (`self.HitCheck`)
              (`SceneComponent.SetHiddenInGame` (`self.Hitbox`) false false)))
          (else
            (`SceneComponent.SetHiddenInGame` (`self.Hitbox`) true false)))))
    (else
      (`self.UpdateAnimation`))))

(event `Reset Combo`
  (set `self.ComboCount` 0)
  (goto _label_2 :!via `Reset`))

(event `self.ReceiveAnyDamage`
  (params (Damage :type "Float (single-precision)") (DamageType :type "DamageType Object Reference") (InstigatedBy :type "Controller Object Reference") (DamageCauser :type "Actor Object Reference"))
  (bind _output_get (set `self.Health` (- (`self.Health`) Damage)))
  (if (<= _output_get 0.0)
    (`PaperFlipbookComponent.SetFlipbook` (`self.Sprite`) "/Game/HeartSteelHorizon/Sprites/Player/FlipBooks/FB_PlayerDeath.FB_PlayerDeath")
    (`PaperFlipbookComponent.SetLooping` (`self.Sprite`) false)
    (set `self.IsDead` true)
    (else
      (`PaperFlipbookComponent.SetFlipbook` (`self.Sprite`) "/Game/HeartSteelHorizon/Sprites/Player/FlipBooks/FB_PlayerHurt.FB_PlayerHurt")
      (`PaperFlipbookComponent.SetLooping` (`self.Sprite`) false))))

(fn `HitCheck`
  (locals (HitSomething :type Boolean))
  (for _array_element (`PrimitiveComponent.GetOverlappingActors` (`self.Hitbox`) "/Game/HeartSteelHorizon/Blueprints/Characters/BP_Player.BP_Player_C")
    (if (!= _array_element self)
      (`GameplayStatics.ApplyDamage` _array_element (`self.DamageAmount`))
      (set `local.HitSomething` true)))
  (if (`local.HitSomething`)
    (`GameplayStatics.SpawnEmitterAtLocation` "/Engine/Tutorial/SubEditors/TutorialAssets/TutorialParticleSystem.TutorialParticleSystem" (`SceneComponent.GetSocketLocation` (`self.Sprite`) "HitPos"))
    (`GameplayStatics.PlaySound2D` "/Engine/EditorSounds/GamePreview/StartPlayInEditor.StartPlayInEditor" 1.0 1.0 0.0 null null)))

(fn `RestartAnimation`
  (`PaperFlipbookComponent.SetLooping` (`self.Sprite`) true)
  (if (not (`PaperFlipbookComponent.IsPlaying` (`self.Sprite`)))
    (`PaperFlipbookComponent.Play` (`self.Sprite`))))

(fn `UpdateAnimation`
  (bind (_returnvalue_x _returnvalue_y _returnvalue_z) (`KismetMathLibrary.BreakVector` (`self.GetVelocity`)))
  (if (`NavMovementComponent.IsMovingOnGround` (`self.CharacterMovement`))
    (if (> (`KismetMathLibrary.VSize` (`MovementComponent.Velocity` (`self.CharacterMovement`))) 0.0)
      (`PaperFlipbookComponent.SetFlipbook` (`self.Sprite`) "/Game/HeartSteelHorizon/Sprites/Player/FlipBooks/FB_PlayerRun.FB_PlayerRun")
      (else
        (`PaperFlipbookComponent.SetFlipbook` (`self.Sprite`) "/Game/HeartSteelHorizon/Sprites/Player/FlipBooks/FB_PlayerIdle.FB_PlayerIdle")))
    (elif (< _returnvalue_z 0.0)
      (`PaperFlipbookComponent.SetFlipbook` (`self.Sprite`) "/Game/HeartSteelHorizon/Sprites/Player/FlipBooks/FB_PlayerFall.FB_PlayerFall")
      (else
        (`PaperFlipbookComponent.SetFlipbook` (`self.Sprite`) "/Game/HeartSteelHorizon/Sprites/Player/FlipBooks/FB_PlayerFallUp.FB_PlayerFallUp")))))

(fn `UserConstructionScript`)